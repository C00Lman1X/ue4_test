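; Collectible item actor that takes a cube or sphere shape, with an arrow that bobs on Tick.
; BeginPlay sets the mesh from the item's type, randomly resolving Unknown to cube or sphere.
; A looping counter feeds a sine into the arrow's relative Z offset, and overlap begin and end each toggle the arrow's visibility.
; OnCollected destroys the actor, logs its type and returns false.
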(event `self.ReceiveActorBeginOverlap`
  (params (OtherActor :type "Actor Object Reference"))
  (`SceneComponent.ToggleVisibility` (`self.Arrow`) false))

(event `self.ReceiveBeginPlay`
  (bind _staticmeshcomponent (`self.StaticMeshComponent`))
  (switch `EItemType` (`self.GetType`)
    (:`IT_Cube`
      (`StaticMeshComponent.SetStaticMesh` _staticmeshcomponent "/Game/StarterContent/Shapes/Shape_Cube.Shape_Cube" :!label _label)
      (`self.SetType` "IT_Cube"))
    (:`IT_Sphere`
      (`StaticMeshComponent.SetStaticMesh` _staticmeshcomponent "/Game/StarterContent/Shapes/Shape_Sphere.Shape_Sphere" :!label _label_2)
      (`self.SetType` "IT_Sphere"))
    (:`IT_Unknown`
      (if (`KismetMathLibrary.RandomBool`)
        (goto _label)
        (else
          (goto _label_2))))))

(event `self.ReceiveActorEndOverlap`
  (params (OtherActor :type "Actor Object Reference"))
  (`SceneComponent.ToggleVisibility` (`self.Arrow`) false))

(event `self.ReceiveTick`
  (params (DeltaSeconds :type "Float (single-precision)"))
  (bind _output_get (set `self.i` (+ (`self.i`) 1)))
  (if (> _output_get 360)
    (set `self.i` 0))
  (`SceneComponent.K2_AddRelativeLocation` (`self.Arrow`) (`KismetMathLibrary.MakeVector` 0.0 0.0 (`KismetMathLibrary.DegSin` (`KismetMathLibrary.Conv_IntToDouble` _output_get))) false false))

(fn `OnCollected`
  (params (character :type "Character Object Reference"))
  (returns (ReturnValue :type Boolean))
  (`self.K2_DestroyActor`)
  (`KismetSystemLibrary.PrintString` (`|GetEnumeratorNameAsString` (`self.GetType`)) false)
  (return false))

(fn `UserConstructionScript`
  (set `self.i` 0))