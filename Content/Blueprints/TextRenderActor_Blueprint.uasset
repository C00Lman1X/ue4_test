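; A door actor that opens when the FirstCppCharacter overlapping it holds enough cubes and spheres.
; Both required counts are randomized at BeginPlay and written to a TextRender, whose visibility toggles on overlap begin and end.
; Meeting them shows a green success message and sets CanBeOpened, which ending overlap clears.
; Tick swings DoorMesh one degree per frame toward -90 or 0 yaw, so speed depends on frame rate.
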(event `self.ReceiveBeginPlay`
  (bind _output_get (set `self.CubesNeeded` (`KismetMathLibrary.RandomInteger` 7)))
  (bind _output_get_2 (set `self.SpheresNeeded` (`KismetMathLibrary.RandomInteger` 7)))
  (`TextRenderComponent.K2_SetText` (`self.TextRender`) (`|FormatText` "Need {S} Sphere(s) and {C} Cube(s)" (`KismetTextLibrary.Conv_IntToText` _output_get_2) (`KismetTextLibrary.Conv_IntToText` _output_get))))

(event `self.ReceiveActorBeginOverlap`
  (params (OtherActor :type "Actor Object Reference"))
  (bind _textrender (`self.TextRender`))
  (`SceneComponent.ToggleVisibility` (`self.TextRender`) false)
  (bind _asfirst_cpp_character (cast `FirstCppCharacter` OtherActor))
  (if (and (>= (`FirstCppCharacter.GetCubes` _asfirst_cpp_character) (`self.CubesNeeded`)) (>= (`FirstCppCharacter.GetSpheres` _asfirst_cpp_character) (`self.SpheresNeeded`)))
    (`TextRenderComponent.K2_SetText` _textrender (`|FormatText` "Well done!"))
    (`TextRenderComponent.SetTextRenderColor` _textrender (`KismetMathLibrary.Conv_LinearColorToColor` (struct :`R` 0.240281 :`G` 1.0 :`B` 0.179989 :`A` 1.0)))
    (set `self.CanBeOpened` true)))

(event `self.ReceiveActorEndOverlap`
  (params (OtherActor :type "Actor Object Reference"))
  (`SceneComponent.ToggleVisibility` (`self.TextRender`) false)
  (set `self.CanBeOpened` false))

(event `self.ReceiveTick`
  (params (DeltaSeconds :type "Float (single-precision)"))
  (`self.Animate` (`self.CanBeOpened`)))

(fn `Animate`
  (params (open :type Boolean))
  (bind _yaw (.yaw (`SceneComponent.RelativeRotation` (`self.DoorMesh`))))
  (if open
    (if (> _yaw -90.0)
      (`SceneComponent.K2_AddRelativeRotation` (`self.DoorMesh`) (`KismetMathLibrary.MakeRotator` 0.0 0.0 (`KismetMathLibrary.Conv_IntToDouble` (`KismetMathLibrary.SelectInt` -1 1 open))) false false :!label _label))
    (elif (< _yaw 0.0)
      (goto _label))))

(fn `UserConstructionScript`)